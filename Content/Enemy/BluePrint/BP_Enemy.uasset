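; BP_Enemy is an enemy character with health tracked by an EnemyStatus object and shown on a floating WBP_EnemyBar widget.
; The bar is initialized with that status on BeginPlay and rotated toward the player camera every tick.
; Capsule overlap with a Sowrd actor applies damage and plays the hit montage.
; Keys 1 and 2 are debug inputs for printing HP and applying test damage, and UpdateWalkSpeed sets max walk speed.
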(event OnComponentBeginOverlap(CapsuleComponent)
  (params (OverlappedComponent :type Primitive%20Component%20Object%20Reference) (OtherActor :type Actor%20Object%20Reference) (OtherComp :type Primitive%20Component%20Object%20Reference) (OtherBodyIndex :type Integer) (bFromSweep :type Boolean) (SweepResult :type Hit%20Result%20Structure%20%28by%20ref%29))
  (Utilities|Casting|CastToSowrd OtherActor)
  (Class|EnemyStatus|EnemyonDamage (Variables|Default|GetEnemyStatus) (Variables|Default|GetTeetEnemyDamage))
  (Animation|StopAnimMontage 0)
  (Animation|Montage|PlayMontage (Variables|Character|GetMesh) "/Game/Enemy/Animateion/AnimationMontage/AMP_Hit.AMP_Hit"))

(event EventBeginPlay
  (bind _aswbp_enemy_bar (Utilities|Casting|CastToWBP_EnemyBar (UserInterface|GetUserWidgetObject (Variables|Default|GetWidget))))
  (Default|InitEnemyBar _aswbp_enemy_bar (Variables|Default|GetEnemyStatus)))

(event EventTick
  (params (DeltaSeconds :type Float%20%28single-precision%29))
  (bind _widget (Variables|Default|GetWidget))
  (Transformation|SetWorldRotation _widget (Math|Rotator|FindLookatRotation (Transformation|GetWorldLocation _widget) (Camera|GetCameraLocation (Game|GetPlayerCameraManager 0))) false false))

(event Input|KeyboardEvents|1
  (params (Key :type Key%20Structure :default "None"))
  ;[0 0 0 0.5] テスト敵ダメージ
  (:Pressed
    (Development|PrintString (Utilities|String|ToString(Float) (Variables|/Script/ActionGame.EnemyStatus|GetEnemyCurrentHP (Variables|Default|GetEnemyStatus))))))

(event Input|KeyboardEvents|2
  (params (Key :type Key%20Structure :default "None"))
  ;[0 0 0 0.5] テスト敵ダメージ
  (:Pressed
    (bind _output_get (Variables|Default|SetTeetEnemyDamage 1e+01))
    (Class|EnemyStatus|EnemyonDamage (Variables|Default|GetEnemyStatus) _output_get)
    (Development|PrintString (Utilities|String|ToString(Float) (Variables|/Script/ActionGame.EnemyStatus|GetEnemyCurrentHP (Variables|Default|GetEnemyStatus))))))

(fn ConstructionScript)

(fn UpdateWalkSpeed
  (params (NewWalkSpeed :type Float%20%28double-precision%29))
  (Variables|/Script/Engine.CharacterMovementComponent|SetMaxWalkSpeed (Variables|Character|GetCharacterMovement) NewWalkSpeed))